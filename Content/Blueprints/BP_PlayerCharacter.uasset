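; Player character Blueprint that handles crouch and zoom through Enhanced Input.
; Crouch ends running, sets crouch speed and uses a timeline to shrink the capsule.
; On release, a capsule trace above the camera must be clear to restore walk speed and reverse it; otherwise the character stays crouched, with no retry here.
; Zoom uses a reversible timeline to narrow camera FOV from a clamped base value while held.
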(event Input|EnhancedActionEvents|EnhancedInputActionIA_Crouch
  (params (ActionValue :type Boolean) (ElapsedSeconds :type Float%20%28double-precision%29) (TriggeredSeconds :type Float%20%28double-precision%29) (InputAction :type Input%20Action%20Object%20Reference :default "/Game/Inputs/IA_Crouch.IA_Crouch"))
  (bind _camera (Variables|Default|GetCamera))
  (bind _returnvalue (Transformation|GetWorldLocation _camera))
  (:Started
    (Class|CoreCharacter|EndRun)
    (Variables|/Script/Engine.CharacterMovementComponent|SetMaxWalkSpeed (Variables|Character|GetCharacterMovement) (Class|CoreCharacter|GetCrouchSpeed))
    (Class|CoreCharacter|SetCrouch true)
    (bind _alpha (Timeline|A_Crouch Play)
      (:Update
        (Components|Capsule|SetCapsuleSize (Variables|Default|GetCapsuleComponent) (Math|Float|Lerp 45.0 22.0 _alpha) (Math|Float|Lerp 9e+01 22.0 _alpha) true))))
  (:Completed
    (bind _returnvalue_2 (Collision|CapsuleTraceByChannel _returnvalue (+ _returnvalue "0.000000,0.000000,96.000000") 45.0 9e+01 "TraceTypeQuery1" false 0 "None"))
    (if (not _returnvalue_2)
      (Variables|/Script/Engine.CharacterMovementComponent|SetMaxWalkSpeed (Variables|Character|GetCharacterMovement) (Class|CoreCharacter|GetWalkSpeed))
      (Class|CoreCharacter|SetCrouch false)
      (Timeline|A_Crouch Reverse))))

(event Input|EnhancedActionEvents|EnhancedInputActionIA_Zoom
  (params (ActionValue :type Boolean) (ElapsedSeconds :type Float%20%28double-precision%29) (TriggeredSeconds :type Float%20%28double-precision%29) (InputAction :type Input%20Action%20Object%20Reference :default "/Game/Inputs/IA_Zoom.IA_Zoom"))
  (bind _returnvalue (Class|CoreCharacter|GetCameraFOV))
  (bind _returnvalue_2 (Math|Float|Clamp(Float) _returnvalue 75.0 1.2e+02))
  (:Started
    (Class|CoreCharacter|SetZooming true)
    (bind _alpha (Timeline|A_Zoom Play)
      (:Update
        (Camera|SetFieldOfView (Variables|Default|GetCamera) (Math|Float|Lerp _returnvalue_2 (/ _returnvalue_2 1.5) _alpha)))))
  (:Completed
    (Class|CoreCharacter|SetZooming false)
    (Timeline|A_Zoom Reverse)))

(fn ConstructionScript)